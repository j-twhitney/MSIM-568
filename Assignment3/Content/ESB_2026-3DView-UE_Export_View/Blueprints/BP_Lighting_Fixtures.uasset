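; Blueprint that lays out downlight fixtures with point lights along a spline for the bottom-floor east hallway.
; The construction script steps along the spline at a configurable spacing, adding a reflector downlight static mesh at each point.
; Each fixture gets a point light at the same horizontal position with a height offset and a configurable intensity.
; The event graph holds no active logic.
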(fn `UserConstructionScript`
  (bind _bottomfloorhallwayeast (`self.BottomFloorHallwayEast`))
  (bind _spacing (`self.Spacing`))
  (for _index (range (+ (`KismetMathLibrary.FFloor` (/ (`SplineComponent.GetSplineLength` _bottomfloorhallwayeast) _spacing)) 1))
    (bind _returnvalue (`SplineComponent.GetLocationAtDistanceAlongSpline` _bottomfloorhallwayeast (* _index _spacing) "Local"))
    (bind _returnvalue_2 (`AddComponent|NODE_AddStaticMeshComponent-0` :`RelativeTransform` (`KismetMathLibrary.MakeTransform` _returnvalue)))
    (`StaticMeshComponent.SetStaticMesh` _returnvalue_2 "/Game/ESB_2026-3DView-UE_Export_View/Geometries/Lighting_Fixtures_J1_-_8_Open_Reflector_Downlight_-_277_J1_-_2_CF18W.Lighting_Fixtures_J1_-_8_Open_Reflector_Downlight_-_277_J1_-_2_CF18W")
    (bind _returnvalue_3 (`AddComponent|NODE_AddPointLightComponent-0` :`RelativeTransform` (`KismetMathLibrary.MakeTransform` (+ (.z _returnvalue) (`KismetMathLibrary.MakeVector` (.x _returnvalue) (.y _returnvalue) (`self.Offset`))))))
    (`LightComponent.SetIntensity` _returnvalue_3 (`self.New Intensity`))))